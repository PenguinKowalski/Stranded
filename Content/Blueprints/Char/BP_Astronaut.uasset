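; Physics-driven astronaut character that steers and thrusts by applying local-space torque and force to its capsule.
; Look input sets pitch and yaw, and rotate input adds roll.
; Thrust burns Fuel, then falls back on Oxygen, which also drains every tick.
; Releasing launch respawns the stored GrabbableItem ahead and fires it with an impulse scaled by clamped hold time, recoiling the astronaut equally backward.
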(event Input|EnhancedActionEvents|EnhancedInputActionIA_Launch
  (params (ActionValue :type Boolean) (ElapsedSeconds :type Float%20%28double-precision%29) (TriggeredSeconds :type Float%20%28double-precision%29) (InputAction :type Input%20Action%20Object%20Reference :default "/Game/Blueprints/Input/IA_Launch.IA_Launch"))
  (bind _returnvalue (Math|Float|Clamp(Float) ElapsedSeconds))
  (bind _capsule (Variables|Default|GetCapsule))
  (bind _launchmultiplier (Variables|Default|GetLaunchMultiplier))
  (bind _returnvalue_2 (Transformation|GetWorldTransform _capsule))
  (bind _returnvalue_3 (Math|Vector|GetForwardVector _capsule))
  (bind (_location _rotation _scale) (Math|Transform|BreakTransform _returnvalue_2))
  (bind _returnvalue_4 (* _returnvalue_3 _returnvalue _launchmultiplier))
  (:Completed
    (if (Utilities|IsValid (Variables|Default|GetObjectToLaunch))
      (Development|PrintString (Utilities|String|ToString(Float) ElapsedSeconds))
      (Rendering|SetActorHiddenInGame (Variables|Default|GetObjectToLaunch) false)
      (Transformation|SetActorTransform (Variables|Default|GetObjectToLaunch) (Math|Transform|MakeTransform (+ _location (* _returnvalue_3 (Variables|Default|GetDistanceSpawn))) _rotation _scale))
      (bind _asgrabbable_item (Utilities|Casting|CastToGrabbableItem (Variables|Default|GetObjectToLaunch)))
      (Class|PrimitiveComponent|SetAllPhysicsAngularVelocityinDegrees (Variables|/Game/Blueprints/PickUp_System/GrabbableItem.GrabbableItem_C|GetCylinder _asgrabbable_item) (Math|Vector|VectorZero) false)
      (Class|PrimitiveComponent|SetAllPhysicsLinearVelocity (Variables|/Game/Blueprints/PickUp_System/GrabbableItem.GrabbableItem_C|GetCylinder _asgrabbable_item) "0, 0, 0" false)
      (Physics|AddImpulse (Variables|/Game/Blueprints/PickUp_System/GrabbableItem.GrabbableItem_C|GetCylinder _asgrabbable_item) _returnvalue_4 "None" true)
      (Physics|AddImpulse _capsule (* _returnvalue_4 -1.0) "None" true)
      (Variables|Default|SetObjectToLaunch (Variables|Default|Getnull)))))

(event Input|EnhancedActionEvents|EnhancedInputActionIA_Force
  (params (ActionValue :type Boolean) (ElapsedSeconds :type Float%20%28double-precision%29) (TriggeredSeconds :type Float%20%28double-precision%29) (InputAction :type Input%20Action%20Object%20Reference :default "/Game/Blueprints/Input/IA_Force.IA_Force"))
  (bind _capsule (Variables|Default|GetCapsule))
  (if (> (Variables|Default|GetFuel) 0.0)
    (Variables|Default|SetFuel (- (Variables|Default|GetFuel) (stale EventTick DeltaSeconds)))
    (Physics|AddForce _capsule (Math|Transform|TransformDirection (Transformation|GetRelativeTransform _capsule) (Math|Vector|MakeVector (* ActionValue (Variables|Default|GetForceO2)) 0.0 0.0)) "None" true :!label _label)
    (elif (> (Variables|Default|GetOxygen) 0.0)
      (Variables|Default|SetOxygen (- (Variables|Default|GetOxygen) (stale EventTick DeltaSeconds)))
      (goto _label))))

(event Input|EnhancedActionEvents|EnhancedInputActionIA_Look
  (params (ActionValue :type Vector%202D%20Structure) (ElapsedSeconds :type Float%20%28double-precision%29) (TriggeredSeconds :type Float%20%28double-precision%29) (InputAction :type Input%20Action%20Object%20Reference :default "/Game/FirstPerson/Input/Actions/IA_Look.IA_Look"))
  (bind _multiply (Variables|Default|GetMultiply))
  (bind _capsule (Variables|Default|GetCapsule))
  (Class|PrimitiveComponent|AddTorqueinDegrees _capsule (Math|Transform|TransformDirection (Transformation|GetRelativeTransform _capsule) (Math|Vector|MakeVector (* (/ _multiply 2.0) (Variables|Default|GetrotationY)) (* (.y ActionValue) _multiply) (* (.x ActionValue) _multiply))) "None" true))

(event Input|EnhancedActionEvents|EnhancedInputActionIA_Rotate
  (params (ActionValue :type Float%20%28double-precision%29) (ElapsedSeconds :type Float%20%28double-precision%29) (TriggeredSeconds :type Float%20%28double-precision%29) (InputAction :type Input%20Action%20Object%20Reference :default "/Game/Blueprints/Input/IA_Rotate.IA_Rotate"))
  (bind _multiply (Variables|Default|GetMultiply))
  (bind _capsule (Variables|Default|GetCapsule))
  (:Triggered
    (Variables|Default|SetrotationY ActionValue)
    (Class|PrimitiveComponent|AddTorqueinDegrees _capsule (Math|Transform|TransformDirection (Transformation|GetRelativeTransform _capsule) (Math|Vector|MakeVector (* (/ _multiply 2.0) (Variables|Default|GetrotationY)) (* (.y (stale Input|EnhancedActionEvents|EnhancedInputActionIA_Look ActionValue)) _multiply) (* (.x (stale Input|EnhancedActionEvents|EnhancedInputActionIA_Look ActionValue)) _multiply))) "None" true))
  (:Canceled
    (Variables|Default|SetrotationY 0.0 :!label _label))
  (:Completed
    (goto _label)))

(event EventBeginPlay)

(event Collision|EventActorBeginOverlap
  (params (OtherActor :type Actor%20Object%20Reference)))

(event EventTick
  (params (DeltaSeconds :type Float%20%28single-precision%29))
  (Variables|Default|SetOxygen (- (Variables|Default|GetOxygen) DeltaSeconds)))

(fn ConstructionScript)