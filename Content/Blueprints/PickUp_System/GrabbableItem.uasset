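; GrabbableItem is a pickup that the player's BP_Astronaut can grab and carry, registering itself as that astronaut's ObjectToLaunch.
; Sphere overlaps toggle CanPickup, which lets IA_Action store the astronaut and set Picked.
; While Picked, Tick snaps the Cylinder to an offset in front of the astronaut's capsule, matching its rotation.
; Nodes disabling the Cylinder's collision and physics are unconnected, and the graph never clears Picked.
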(event OnComponentBeginOverlap(Sphere)
  (params (OverlappedComponent :type Primitive%20Component%20Object%20Reference) (OtherActor :type Actor%20Object%20Reference) (OtherComp :type Primitive%20Component%20Object%20Reference) (OtherBodyIndex :type Integer) (bFromSweep :type Boolean) (SweepResult :type Hit%20Result%20Structure%20%28by%20ref%29))
  (Variables|Default|SetcanPickup true))

(event OnComponentEndOverlap(Sphere)
  (params (OverlappedComponent :type Primitive%20Component%20Object%20Reference) (OtherActor :type Actor%20Object%20Reference) (OtherComp :type Primitive%20Component%20Object%20Reference) (OtherBodyIndex :type Integer))
  (Variables|Default|SetcanPickup false))

(event Input|EnhancedActionEvents|EnhancedInputActionIA_Action
  (params (ActionValue :type Boolean) (ElapsedSeconds :type Float%20%28double-precision%29) (TriggeredSeconds :type Float%20%28double-precision%29) (InputAction :type Input%20Action%20Object%20Reference :default "/Game/Blueprints/Input/IA_Action.IA_Action"))
  (if (Variables|Default|GetcanPickup)
    (bind _asbp_astronaut (Utilities|Casting|CastToBP_Astronaut (Game|Player|GetPlayerPawn 0)))
    (Variables|Default|Setchar _asbp_astronaut)
    (Variables|/Game/Blueprints/Char/BP_Astronaut.BP_Astronaut_C|SetObjectToLaunch _asbp_astronaut self)
    (Variables|Default|Setpicked true)))

(event EventBeginPlay)

(event EventTick
  (params (DeltaSeconds :type Float%20%28single-precision%29))
  (bind _char (Variables|Default|Getchar))
  (bind _capsule (Variables|/Game/Blueprints/Char/BP_Astronaut.BP_Astronaut_C|GetCapsule _char))
  (if (Variables|Default|Getpicked)
    (Transformation|SetWorldLocationAndRotation (Variables|Default|GetCylinder) (+ (Transformation|GetWorldLocation _capsule) (* (Math|Vector|GetForwardVector _capsule) (Variables|Default|GetoffsetLocation))) (Transformation|GetWorldRotation _capsule) false false)))

(fn ConstructionScript)